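; Manager actor that sets up and runs a ray-plane intersection test.
; On BeginPlay it spawns a plane, an intersection algorithm actor and a test pawn at hardcoded transforms.
; Each Tick it rotates the pawn by a fixed step, then passes the pawn's origin and normal as a ray, with the plane, to the algorithm.
; The hit result feeds an empty branch, and the debug prints are disconnected.
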(event EventBeginPlay
  (bind _returnvalue (Game|SpawnActorfromClass "/Game/PlaneClass_BP.PlaneClass_BP_C" (Math|Transform|MakeTransform (Math|Vector|MakeVector -7.1e+02 8.9e+03 1.1e+02)) "Undefined" 0 0))
  (bind _output_get (Variables|Default|SetPlane_Obj _returnvalue))
  (bind _returnvalue_2 (Game|SpawnActorfromClass "/Script/IntersectionTests.IntersectionTestAlgorithm" (Math|Transform|MakeTransform "0, 0, 0") "Undefined" 0 0))
  (Variables|Default|SetTestAlgo_Obj _returnvalue_2)
  (bind _returnvalue_3 (Game|SpawnActorfromClass "/Script/IntersectionTests.IntersectionTestsPawn" (Math|Transform|MakeTransform "-680.000000,7510.000000,112.769867" "0,90.000000, 0") "Undefined" 0 0))
  (Variables|Default|SetIntersectionPawn_Obj _returnvalue_3))

(event Collision|EventActorBeginOverlap
  (params (OtherActor :type Actor%20Object%20Reference)))

(event EventTick
  (params (DeltaSeconds :type Float%20%28single-precision%29))
  (bind _intersectionpawn_obj (Variables|Default|GetIntersectionPawn_Obj))
  (Class|Actor|AddActorWorldRotation _intersectionpawn_obj "0,2.000000, 0")
  (bind _returnvalue (Class|IntersectionTestsPawn|GetPawnOrigin _intersectionpawn_obj))
  (bind _returnvalue_2 (Class|IntersectionTestsPawn|GetPawnNormal _intersectionpawn_obj))
  (bind _returnvalue_3 (Class|IntersectionTestAlgorithm|DoesRayPlaneIntersect (Variables|Default|GetTestAlgo_Obj) (Variables|Default|GetPlane_Obj) _returnvalue _returnvalue_2))
  (if _returnvalue_3
    _))

(fn ConstructionScript)