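; PlaneClass_BP is an actor that spins by a fixed step each tick and visualizes a plane with debug drawing.
; Tick stores PlaneOrigin above the root and PlaneNormal as that origin plus the forward vector, all scaled, so the normal is not a pure direction.
; It draws a plane facing the root's forward vector at the raised point, plus an arrow from there to the same scaled value.
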(event EventBeginPlay)

(event Collision|EventActorBeginOverlap
  (params (OtherActor :type Actor%20Object%20Reference)))

(event EventTick
  (params (DeltaSeconds :type Float%20%28single-precision%29))
  (bind _defaultsceneroot (Variables|Default|GetDefaultSceneRoot))
  (bind _defaultsceneroot_2 (Variables|Default|GetDefaultSceneRoot))
  (bind _returnvalue (Transformation|GetWorldLocation _defaultsceneroot))
  (bind _returnvalue_2 (Transformation|GetWorldRotation _defaultsceneroot_2))
  (bind _returnvalue_3 (Math|Vector|GetForwardVector _returnvalue_2))
  (bind _returnvalue_4 (+ _returnvalue "0, 0,500.000000"))
  (bind _returnvalue_5 (+ _returnvalue_4 _returnvalue_3))
  (bind _returnvalue_6 (* _returnvalue_5 1e+03))
  (Class|Actor|AddActorWorldRotation "0.000000,2.000000, 0")
  (Variables|Default|SetplaneOrigin _returnvalue_4)
  (Variables|Default|SetplaneNormal _returnvalue_6)
  (Class|KismetSystemLibrary|DrawDebugPlane (Class|KismetMathLibrary|MakePlanefromPointandNormal _returnvalue _returnvalue_3) _returnvalue_4 5e+02 "(R=1.000000,G=1.000000,B=1.000000,A=1.000000)" 0.1)
  (Rendering|Debug|DrawDebugArrow _returnvalue_4 _returnvalue_6 0.0 "(R=0.779167,G=0.344750,B=0.734387,A=1.000000)" 0.2 3.0))

(fn ConstructionScript)