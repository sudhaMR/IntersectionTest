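; RayPlaneManager_BP is a manager actor that demonstrates ray-plane and ray-AABB intersection tests.
; On BeginPlay it spawns a plane, a box, a test-algorithm actor and a ray-source pawn at hard-coded transforms.
; Each Tick it yaws the pawn, reads its ray origin, normal and end, and passes them to the algorithm actor.
; Any hit on the plane or box is drawn as a short-lived debug point.
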(event EventBeginPlay
  (bind _returnvalue (Game|SpawnActorfromClass "/Game/PlaneClass_BP.PlaneClass_BP_C" (Math|Transform|MakeTransform "-710.000000,8900.000000,-3000.000000" "0,90.000000, 0") "Undefined" 0 0))
  (bind _output_get (Variables|Default|SetPlane_Obj _returnvalue))
  (bind _returnvalue_2 (Game|SpawnActorfromClass "/Script/IntersectionTests.IntersectionTestAlgorithm" (Math|Transform|MakeTransform "0, 0, 0") "Undefined" 0 0))
  (Variables|Default|SetTestAlgo_Obj _returnvalue_2)
  (bind _returnvalue_3 (Game|SpawnActorfromClass "/Script/IntersectionTests.IntersectionTestsPawn" (Math|Transform|MakeTransform "-680.000000,7510.000000,300.000000" "0,90.000000, 0") "Undefined" 0 0))
  (Variables|Default|SetIntersectionPawn_Obj _returnvalue_3)
  (bind _returnvalue_4 (Game|SpawnActorfromClass "/Game/AABBClass_BP.AABBClass_BP_C" (Math|Transform|MakeTransform "-1410.000000,5388.000000,580.000000") "Undefined" 0 0))
  (Variables|Default|SetAABBObj _returnvalue_4))

(event Collision|EventActorBeginOverlap
  (params (OtherActor :type Actor%20Object%20Reference)))

(event EventTick
  (params (DeltaSeconds :type Float%20%28single-precision%29))
  (bind _intersectionpawn_obj (Variables|Default|GetIntersectionPawn_Obj))
  (bind _testalgo_obj (Variables|Default|GetTestAlgo_Obj))
  (bind _testalgo_obj_2 (Variables|Default|GetTestAlgo_Obj))
  (Class|Actor|AddActorWorldRotation _intersectionpawn_obj "0,0.500000, 0")
  (bind _returnvalue (Class|IntersectionTestsPawn|GetPawnOrigin _intersectionpawn_obj))
  (Variables|Default|SetRayOrigin _returnvalue)
  (bind _returnvalue_2 (Class|IntersectionTestsPawn|GetPawnNormal _intersectionpawn_obj))
  (Variables|Default|SetRayNormal _returnvalue_2)
  (bind _returnvalue_3 (Class|IntersectionTestsPawn|GetPawnEnd _intersectionpawn_obj))
  (Variables|Default|SetRayEnd _returnvalue_3)
  (bind _returnvalue_4 (Class|IntersectionTestAlgorithm|DoesRayPlaneIntersect _testalgo_obj_2 (Variables|Default|GetPlane_Obj) (Variables|Default|GetRayOrigin) (Variables|Default|GetRayNormal) (Variables|Default|GetRayEnd)))
  (bind _returnvalue_5 (Class|IntersectionTestAlgorithm|DoesRayAABBIntersect _testalgo_obj_2 (Variables|Default|GetRayOrigin) (Variables|Default|GetRayEnd) (Variables|Default|GetAABBObj)))
  (Utilities|FlowControl|Sequence
    (:then_0
      (if _returnvalue_4
        (Rendering|Debug|DrawDebugPoint (Variables|/Script/IntersectionTests.IntersectionTestAlgorithm|GetPlaneIntersectionPoint _testalgo_obj) 6e+01 "(R=0.000000,G=0.822152,B=1.000000,A=1.000000)" 0.05)))
    (:then_1
      (if _returnvalue_5
        (Rendering|Debug|DrawDebugPoint (Variables|/Script/IntersectionTests.IntersectionTestAlgorithm|GetAABBIntersectionPoint _testalgo_obj) 1e+01 "(R=0.067542,G=0.014493,B=0.479167,A=1.000000)" 0.5)))))

(fn ConstructionScript)