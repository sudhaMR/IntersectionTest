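; AABBClass_BP is a debug actor that sets up and visualises a bounding box, apparently an AABB test.
; BeginPlay captures the actor location and a fixed cubic extent, then passes both to SetMinMax, which is defined outside this graph.
; Tick yaws the actor by a constant per-frame step and draws a short-lived debug box using the root's rotation, while SetMinMax is never called again.
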(event EventBeginPlay
  (bind _output_get (Variables|Default|SetDebugBoxOrigin (Transformation|GetActorLocation)))
  (bind _output_get_2 (Variables|Default|SetDebugBoxExtent "1000.000000,1000.000000,1000.000000"))
  (Class|AABBClass|SetMinMax _output_get _output_get_2))

(event Collision|EventActorBeginOverlap
  (params (OtherActor :type Actor%20Object%20Reference)))

(event EventTick
  (params (DeltaSeconds :type Float%20%28single-precision%29))
  (Class|Actor|AddActorWorldRotation "0,1.000000, 0")
  (Rendering|Debug|DrawDebugBox :Center (Variables|Default|GetDebugBoxOrigin) :Extent (Variables|Default|GetDebugBoxExtent) :Rotation (Transformation|GetWorldRotation (Variables|Default|GetDefaultSceneRoot)) :Duration 0.08 :Thickness 15.0))

(fn ConstructionScript)